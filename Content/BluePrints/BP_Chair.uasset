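; BP_Chair is a Blueprint actor that destroys itself when another actor overlaps it.
; On BeginPlay it gathers all actors in the level and prints the display name of one at a hard-coded array index.
; Disconnected practice graphs sum numbers from 1 to 100 (evens, odds, multiples, all) and search static mesh actors for "Floor", but never run.
; Tick, the construction script and NewFunction_0 are empty.
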(event EventBeginPlay
  (bind _outactors (Actor|GetAllActorsOfClass "/Script/Engine.Actor"))
  (Development|PrintString (Utilities|GetDisplayName (Utilities|Array|Get(acopy) _outactors 13))))

(event Collision|EventActorBeginOverlap
  (params (OtherActor :type Actor%20Object%20Reference))
  (Actor|DestroyActor))

(event EventTick
  (params (DeltaSeconds :type Float%20%28single-precision%29)))

(fn ConstructionScript)

(fn NewFunction0)