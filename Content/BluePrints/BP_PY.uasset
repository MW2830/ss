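; BP_PY is a Blueprint that plays a random 2D sound effect when play begins, apparently doubling as a scratchpad for loop exercises.
; BeginPlay picks one of the first five entries in the sound effect array 효과음리스트.
; Unconnected chains, which never run, practice printing actor names and printing or summing the 숫자 number array.
; Overlap, Tick and the construction script are empty.
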(event EventBeginPlay
  (Audio|PlaySound2D (Utilities|Array|Get(acopy) (Variables|Default|Get효과음리스트) (Math|Random|RandomIntegerinRange 0 4)) 1.0 1.0 0.0 0 0))

(event Collision|EventActorBeginOverlap
  (params (OtherActor :type Actor%20Object%20Reference)))

(event EventTick
  (params (DeltaSeconds :type Float%20%28single-precision%29)))

(fn ConstructionScript)